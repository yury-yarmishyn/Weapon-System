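; BP_TtEnemy is an enemy character Blueprint with a Gameplay Ability System component and an on-screen attribute readout for debugging.
; Every Tick, it loops through all of the component's attributes and prints the actor's display name, the attribute name and its base value.
; The prints use zero duration, so they refresh each frame, and show base values rather than current ones.
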(event `self.ReceiveTick`
  (params (DeltaSeconds :type "Float (single-precision)"))
  (for _array_element (`AbilitySystemComponent.GetAllAttributes` (`self.AbilitySystemComponent`))
    (`KismetSystemLibrary.PrintString` (`KismetStringLibrary.Concat_StrStr` (`KismetSystemLibrary.GetDisplayName` self) " " (`.AttributeName` (break `GameplayAttribute` _array_element)) "" (`KismetStringLibrary.Conv_DoubleToString` (`.ReturnValue` (`AbilitySystemBlueprintLibrary.GetFloatAttributeBaseFromAbilitySystemComponent` (`self.AbilitySystemComponent`) _array_element)))) true true (struct :`G` 0.66 :`B` 1.0 :`A` 1.0) 0.0)))

(fn `UserConstructionScript`)